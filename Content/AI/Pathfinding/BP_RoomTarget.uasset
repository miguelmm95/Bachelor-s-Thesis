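; BP_RoomTarget is an AI pathfinding actor that marks a room target and gathers the child nodes around it.
; Its construction script sizes a sphere component to the Radius variable.
; On BeginPlay it stores the overlapping BP_RoomTargetChildren actors in ChildrenNodes.
; A Visibility sphere trace from the billboard's location runs first, but its result is unused.
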(event `self.ReceiveBeginPlay`
  (`KismetSystemLibrary.SphereTraceSingle` (`SceneComponent.K2_GetComponentLocation` (`self.Billboard`)) (0.0 0.0 0.0) (`self.Radius`) "TraceTypeQuery1")
  (set `self.ChildrenNodes` (`PrimitiveComponent.GetOverlappingActors` (`self.Sphere`) "/Game/AI/Pathfinding/BP_RoomTargetChildren.BP_RoomTargetChildren_C")))

(fn `UserConstructionScript`
  (`SphereComponent.SetSphereRadius` (`self.Sphere`) (`self.Radius`) true))